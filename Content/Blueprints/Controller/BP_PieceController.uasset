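; BP_PieceController is an AI controller that moves a Korean chess piece to a new destination.
; Its PieceMove event runs AIMoveTo without pathfinding and sets the controlled KCPiece's state to MOVE.
; When the move finishes, it returns the piece to IDLE, resets its rotation, and has the KoreanChessGameMode check the current turn.
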(event EventBeginPlay)

(event EventTick
  (params (DeltaSeconds :type Float%20%28single-precision%29)))

(event EventPieceMove
  (params (NewDestination :type Vector :default "0, 0, 0"))
  (bind _returnvalue (Game|GetGameMode))
  (AI|AIMoveTo self NewDestination 0 -1.0 "Disable" "Disable" false true false "Disable"
    (:then
      (bind _askcpiece (Utilities|Casting|CastToKCPiece (Pawn|GetControlledPawn)))
      (Class|KCPiece|SetState _askcpiece "MOVE"))
    (:OnMoveFinished
      (bind _askcpiece_2 (Utilities|Casting|CastToKCPiece (Pawn|GetControlledPawn)))
      (Class|KCPiece|SetState _askcpiece_2 "IDLE")
      (Class|KCPiece|InitializeRotation _askcpiece_2)
      (Utilities|IsValid _returnvalue
        (:Is%20Valid
          (bind _askorean_chess_game_mode (Utilities|Casting|CastToKoreanChessGameMode _returnvalue))
          (Class|KoreanChessGameMode|CheckCurrentTurn _askorean_chess_game_mode "MOVE"))))))

(fn ConstructionScript)