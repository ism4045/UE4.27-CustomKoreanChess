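; BP_KoreanChessGameMode is the game mode for a Korean chess game, handling returns to the lobby or the menu.
; ReturnLobby triggers a loading change and server-travels to LobbyMap.
; ReturnMenu walks player controllers in reverse, telling the one at index 1 to exit the server directly.
; Other controllers destroy the session first, then exit whether that succeeds or fails.
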(event EventBeginPlay)

(event EventTick
  (params (DeltaSeconds :type Float%20%28single-precision%29)))

(event EventReturnLobby
  (Class|KoreanChessGameMode|ChangeLoading)
  (Development|ExecuteConsoleCommand (Utilities|String|Append "servertravel " "LobbyMap") 0))

(event EventReturnMenu
  (bind _returnvalue (Class|KoreanChessGameMode|GetPlayerControllerArray))
  (bind (_arrayindex _arrayelement) (Utilities|Array|ReverseforEachLoop _returnvalue)
    (:LoopBody
      (if (== _arrayindex 1)
        (bind _askorean_chess_player_controller (Utilities|Casting|CastToKoreanChessPlayerController _arrayelement))
        (Class|KoreanChessPlayerController|ExitServer _askorean_chess_player_controller)
        (else
          (|DestroySession _arrayelement
            (:OnSuccess
              _)
            (:OnFailure
              _))
          (bind _askorean_chess_player_controller_2 (Utilities|Casting|CastToKoreanChessPlayerController _arrayelement))
          (Class|KoreanChessPlayerController|ExitServer _askorean_chess_player_controller_2))))))

(fn ConstructionScript)